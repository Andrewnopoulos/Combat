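; MPController is a player controller that lets its player spawn or despawn a character in the combat game.
; Key 1 or gamepad Special Right calls SpawnCharacter on the CombatGameMode, while key 2 or Special Left calls DespawnCharacter, each passing the controller itself.
; It also stores a PlayerIndex exposed through getter and setter functions.
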(event Input|GamepadEvents|GamepadSpecialLeft
  (params (Key :type Key%20Structure :default "AnyKey"))
  (:Pressed
    (bind _ascombat_game_mode (Utilities|Casting|CastToCombatGameMode (Game|GetGameMode)))
    (Default|DespawnCharacter _ascombat_game_mode self)))

(event Input|GamepadEvents|GamepadSpecialRight
  (params (Key :type Key%20Structure :default "AnyKey"))
  (:Pressed
    (bind _ascombat_game_mode (Utilities|Casting|CastToCombatGameMode (Game|GetGameMode)))
    (Default|SpawnCharacter _ascombat_game_mode self)))

(event Input|KeyboardEvents|1
  (params (Key :type Key%20Structure :default "AnyKey"))
  (:Pressed
    (bind _ascombat_game_mode (Utilities|Casting|CastToCombatGameMode (Game|GetGameMode)))
    (Default|SpawnCharacter _ascombat_game_mode self)))

(event Input|KeyboardEvents|2
  (params (Key :type Key%20Structure :default "AnyKey"))
  (:Pressed
    (bind _ascombat_game_mode (Utilities|Casting|CastToCombatGameMode (Game|GetGameMode)))
    (Default|DespawnCharacter _ascombat_game_mode self)))

(fn ConstructionScript)

(fn GetPlayerIndex
  (return (Variables|Default|GetPlayerIndex)))

(fn SetPlayerIndex
  (params (PlayerIndex :type Integer))
  (Variables|Default|SetPlayerIndex PlayerIndex))