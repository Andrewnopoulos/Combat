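; Game mode for local multiplayer combat that creates the players and handles swapping their pawns in and out.
; On begin play it caches the PlayerStarts, creates local players in a counted loop and gives each MPController an index.
; Spawn and despawn events replace a valid pawn with a coloured MPCharacter or an InitPawn, using GetRandomSpawn for placement.
; Both events then point the controller's view at the shared GameCamera.
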(event Custom|SpawnCharacter
  (params (Player%20Controller :type Player%20Controller%20Object%20Reference))
  (bind _returnvalue (Pawn|GetControlledPawn Player%20Controller))
  (Utilities|IsValid _returnvalue
    (:Is%20Valid
      (Actor|DestroyActor _returnvalue)
      (bind _returnvalue_2 (Game|SpawnActorfromClass "/Game/Blueprints/MPCharacter.MPCharacter_C" (Utilities|GetRandomSpawn) "Undefined" 0 0))
      (Pawn|Possess Player%20Controller _returnvalue_2)
      (Default|SetPlayerColour _returnvalue_2)
      (Game|Player|SetViewTargetwithBlend Player%20Controller (Variables|Default|GetGameCamera) 0.0 "VTBlend_Linear" 0.0 false))))

(event Custom|DespawnCharacter
  (params (Player%20Controller :type Player%20Controller%20Object%20Reference))
  (bind _returnvalue (Pawn|GetControlledPawn Player%20Controller))
  (Utilities|IsValid _returnvalue
    (:Is%20Valid
      (Actor|DestroyActor _returnvalue)
      (bind _returnvalue_2 (Game|SpawnActorfromClass "/Game/Blueprints/InitPawn.InitPawn_C" (Utilities|GetRandomSpawn) "Undefined" 0 0))
      (Pawn|Possess Player%20Controller _returnvalue_2)
      (Game|Player|SetViewTargetwithBlend Player%20Controller (Variables|Default|GetGameCamera) 0.0 "VTBlend_Linear" 0.0 false))))

(event EventBeginPlay
  (bind _outactors (Actor|GetAllActorsOfClass "/Script/Engine.PlayerStart"))
  (Variables|Default|SetSpawnPoints _outactors)
  (while (<= (Variables|Default|GetNumberOfPlayers) 3)
    (Variables|Default|SetNumberOfPlayers (+ (Variables|Default|GetNumberOfPlayers) 1))
    (bind _returnvalue (Class|GameplayStatics|CreatePlayer -1))
    (Utilities|Casting|CastToMPController _returnvalue))
  (bind _outactors_2 (Actor|GetAllActorsOfClass "/Game/Blueprints/MPController.MPController_C"))
  (for (_array_element _array_index) _outactors_2
    (Variables|/Game/Blueprints/MPController.MPController_C|SetPlayerIndex _array_element _array_index)))

(fn ConstructionScript)