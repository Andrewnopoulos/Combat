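; Projectile actor that damages what it hits and destroys itself on impact.
; On overlap, damageable actors without the Friendly tag receive Damage through the IDamageable interface's health message.
; Those hits, and overlaps with non-damageable actors, play an explosion sound, spawn laser sparks and destroy the projectile.
; Friendly-tagged damageable actors are ignored, so the projectile survives overlapping them.
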(event Collision|EventActorBeginOverlap
  (params (OtherActor :type Actor%20Object%20Reference))
  (bind _returnvalue (Transformation|GetActorTransform))
  ;[1 1 1] Projectile Damage
  (if (Utilities|DoesObjectImplementInterface OtherActor "/Game/Blueprints/OldAssets/iDamageable.iDamageable_C")
    (if (not (Actor|ActorHasTag OtherActor "Friendly"))
      (Class|IDamageable|AffectHealth(Message) OtherActor (Variables|Default|GetDamage))
      (Audio|SpawnSoundAttached "/Game/StarterContent/Audio/Explosion02.Explosion02" (Variables|Default|GetProjectileCollision) :!label _label)
      (Effects|SpawnEmitteratLocation "/Game/StarterContent/Particles/LaserSparks.LaserSparks" (.location _returnvalue) (.rotation _returnvalue))
      (Actor|DestroyActor))
    (else
      (goto _label))))

(fn ConstructionScript)