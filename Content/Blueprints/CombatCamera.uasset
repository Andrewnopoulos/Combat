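; CombatCamera is a camera actor that follows the group of MPCharacter players from above.
; On BeginPlay it fills ActivePlayers with every MPCharacter in the level, and AddPlayer and RemovePlayer edit that list afterward.
; Each Tick it averages the players' locations and moves itself to that midpoint plus a fixed height offset, without smoothing, zoom or an empty-list check.
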(event EventTick
  (params (DeltaSeconds :type Float%20%28single-precision%29))
  (bind _activeplayers (Variables|Default|GetActivePlayers))
  (Variables|Default|SetCamPosition "0, 0, 0")
  (for _array_element _activeplayers
    (Variables|Default|SetCamPosition (+ (Transformation|GetActorLocation _array_element) (Variables|Default|GetCamPosition))))
  (bind _output_get (Variables|Default|SetCamPosition (/ (Variables|Default|GetCamPosition) (Utilities|Array|Length _activeplayers))))
  (Transformation|SetActorLocation (+ _output_get "0,0.000000,500.000000") false false))

(event EventBeginPlay
  (bind _outactors (Actor|GetAllActorsOfClass "/Game/Blueprints/MPCharacter.MPCharacter_C"))
  (Variables|Default|SetActivePlayers _outactors))

(fn ConstructionScript)

(fn AddPlayer
  (params (newPlayer :type MP%20Character%20Object%20Reference))
  (Utilities|Array|Add (Variables|Default|GetActivePlayers) newPlayer))

(fn RemovePlayer
  (params (player :type MP%20Character%20Object%20Reference))
  (bind _returnvalue (Utilities|Array|RemoveItem (Variables|Default|GetActivePlayers) player))
  (return _returnvalue))